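; Enemy that paces back and forth along world X and takes damage until it is destroyed.
; Tick nudges the capsule using a counter that swings between about -10 and 10, with Delays spacing the counter updates.
; Any damage spawns an impact actor, then shrinks and shifts a static mesh that acts as health, using the player's EnemyDamage.
; The actor destroys itself once that scale, less another hit, reaches a negative threshold.
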(event Custom|reduce_en_hp)

(event EventBeginPlay)

(event Collision|EventActorBeginOverlap
  (params (OtherActor :type Actor%20Object%20Reference)))

(event EventTick
  (params (DeltaSeconds :type Float%20%28single-precision%29))
  (bind _capsulecomponent (Variables|Collision|GetCapsuleComponent))
  (bind _capsulecomponent_2 (Variables|Collision|GetCapsuleComponent))
  (bind _returnvalue (Transformation|GetWorldLocation _capsulecomponent_2))
  (bind _returnvalue_2 (Transformation|GetWorldLocation _capsulecomponent))
  (bind (_x _y _z) (Class|KismetMathLibrary|BreakVector3f _returnvalue))
  (bind (_x_2 _y_2 _z_2) (Class|KismetMathLibrary|BreakVector3f _returnvalue_2))
  (if (Variables|Default|Getok)
    (if (< (Variables|Default|Getx) 10)
      (bind _result (Math|Float|IncrementFloat _x_2)
        (:%20%20
          (Transformation|SetWorldLocation (Variables|Collision|GetCapsuleComponent) (Math|Vector|MakeVector _result _y_2 _z_2) false false)
          (Utilities|FlowControl|Delay 0.1)
          (bind _result_2 (Math|Integer|IncrementInt (Variables|Default|Getx))
            (:%20%20
              (Variables|Default|Setx _result_2)))))
      (else
        (Variables|Default|Setok false)
        (bind _result_3 (Math|Float|DecrementFloat _x :!label _label)
          (:%20%20
            (Transformation|SetWorldLocation (Variables|Collision|GetCapsuleComponent) (Math|Vector|MakeVector _result_3 _y _z) false false)
            (Utilities|FlowControl|Delay 0.1)
            (bind _result_4 (Math|Integer|DecrementInt (Variables|Default|Getx))
              (:%20%20
                (Variables|Default|Setx _result_4)))))))
    (elif (> (Variables|Default|Getx) -10)
      (goto _label)
      (else
        (Variables|Default|Setok true)))))

(event Game|Damage|EventAnyDamage
  (params (Damage :type Float%20%28single-precision%29) (DamageType :type Damage%20Type%20Object%20Reference) (InstigatedBy :type Controller%20Object%20Reference) (DamageCauser :type Actor%20Object%20Reference))
  (bind _staticmesh (Variables|Default|GetStaticMesh))
  (bind _relativescale3d (Variables|/Script/Engine.SceneComponent|GetRelativeScale3D _staticmesh))
  (bind _relativelocation (Variables|/Script/Engine.SceneComponent|GetRelativeLocation _staticmesh))
  (bind (_x _y _z) (Class|KismetMathLibrary|BreakVector3f _relativescale3d))
  (bind (_x_2 _y_2 _z_2) (Class|KismetMathLibrary|BreakVector3f _relativelocation))
  (Game|SpawnActorfromClass "/Game/Blueprints/enemy_impact.enemy_impact_C" (Transformation|GetActorTransform) "Undefined" 0 0)
  (bind _aspaper_2d_char (Utilities|Casting|CastToPaper2d_char (Game|GetPlayerCharacter 0)))
  (Transformation|SetRelativeScale3D _staticmesh (Math|Vector|MakeVector (- _x (/ (Variables|/Game/Blueprints/Paper2d_char.Paper2d_char_C|Getenemy_damage _aspaper_2d_char) 1e+02)) _y _z))
  (Transformation|SetRelativeLocation _staticmesh (Math|Vector|MakeVector _x_2 (- _y_2 5.0) _z_2) false false)
  (Development|PrintString (Utilities|String|ToString(Float) (- _x (/ (Variables|/Game/Blueprints/Paper2d_char.Paper2d_char_C|Getenemy_damage _aspaper_2d_char) 1e+02))))
  (if (<= (- _x (/ (Variables|/Game/Blueprints/Paper2d_char.Paper2d_char_C|Getenemy_damage _aspaper_2d_char) 1e+02)) -0.5)
    (Actor|DestroyActor)))

(fn ConstructionScript)