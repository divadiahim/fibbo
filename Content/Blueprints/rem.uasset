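; The rem Blueprint is a ram charge pickup or trigger that raises the player's Yamete counter when its capsule registers a hit.
; The hit handler checks HitComponent for the "ram_charge" tag, increments the counter on Paper2d_char and passes it to PowerS through Updateram.
; An Ok flag gates the handler, closing after each award and reopening after a 20-second Delay, so the object stays in place as a reusable source.
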(event OnComponentHit(Capsule)
  (params (HitComponent :type Primitive%20Component%20Object%20Reference) (OtherActor :type Actor%20Object%20Reference) (OtherComp :type Primitive%20Component%20Object%20Reference) (NormalImpulse :type Vector :default "0, 0, 0") (Hit :type Hit%20Result%20Structure%20%28by%20ref%29))
  (if (Components|ComponentHasTag HitComponent "ram_charge")
    (if (Variables|Default|Getok)
      (bind _aspaper_2d_char (Utilities|Casting|CastToPaper2d_char (Game|GetPlayerCharacter 0)))
      (bind _result (Math|Integer|IncrementInt (Variables|/Game/Blueprints/Paper2d_char.Paper2d_char_C|Getyamete _aspaper_2d_char))
        (:%20%20
          (bind _output_get (Variables|/Game/Blueprints/Paper2d_char.Paper2d_char_C|Setyamete _aspaper_2d_char _result))
          (Default|Updateram (Variables|/Game/Blueprints/Paper2d_char.Paper2d_char_C|Getpower_s _aspaper_2d_char) _output_get)
          (Variables|Default|Setok false)
          (Utilities|FlowControl|Delay 2e+01)
          (Variables|Default|Setok true))))))

(event EventBeginPlay)

(event Collision|EventActorBeginOverlap
  (params (OtherActor :type Actor%20Object%20Reference)))

(event EventTick
  (params (DeltaSeconds :type Float%20%28single-precision%29)))

(fn ConstructionScript)